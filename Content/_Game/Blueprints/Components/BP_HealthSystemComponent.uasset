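; BP_HealthSystemComponent is an actor component that gives its owning actor health and handles damage and death.
; On BeginPlay it fills health to the maximum and binds to the owner's OnTakeAnyDamage event.
; Each hit lowers clamped health, plays optional sound and Niagara effects at the owner's location, and fires a TookDamage dispatcher, plus a Killed dispatcher at zero health.
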(event Custom|TookDamage
  (params (DamagedActor :type Actor%20Object%20Reference) (Damage :type Float%20%28single-precision%29) (DamageType :type Damage%20Type%20Object%20Reference) (InstigatedBy :type Controller%20Object%20Reference) (DamageCauser :type Actor%20Object%20Reference))
  (Variables|Default|SetCurrentHealth (Math|Float|Clamp(Float) (- (Variables|Default|GetCurrentHealth) Damage) 0.0 (Variables|Default|GetMaxHealth)))
  (CallFunction|PlayFX)
  (Default|CallOnTookDamage Damage)
  (if (<= (Variables|Default|GetCurrentHealth) 0.0)
    (Default|CallOnKilled)))

(event EventBeginPlay
  (Variables|Default|SetOwner (Components|GetOwner))
  (Variables|Default|SetCurrentHealth (Variables|Default|GetMaxHealth))
  (EventDispatchers|BindEventtoOnTakeAnyDamage (Variables|Default|GetOwner) (EventDispatchers|CreateEvent :!event Custom|TookDamage)))

(fn PlayFX
  (bind _damagesound (Variables|Default|GetDamageSound))
  (bind _damageparticles (Variables|Default|GetDamageParticles))
  (Utilities|IsValid _damagesound
    (:Is%20Valid
      (Audio|PlaySoundatLocation _damagesound (Transformation|GetActorLocation (Variables|Default|GetOwner)) "0, 0, 0" 1.0 1.0 0.0 0 0 0 0))
    (:Is%20Not%20Valid
      _))
  (Utilities|IsValid _damageparticles
    (:Is%20Valid
      (Niagara|SpawnSystematLocation _damageparticles (Transformation|GetActorLocation (Variables|Default|GetOwner))))))