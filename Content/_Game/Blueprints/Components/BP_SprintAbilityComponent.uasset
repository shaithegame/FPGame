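; Actor component that gives a character a sprint ability by switching its walk speed.
; StartSprint and StopSprint take a CharacterMovement reference and set MaxWalkSpeed to SprintSpeed or WalkSpeed.
; An IsSprinting flag guards both functions so repeated calls change nothing.
; It has no active event logic, so sprinting only changes when other code calls these functions.
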(event EventBeginPlay)

(event EventTick
  (params (DeltaSeconds :type Float%20%28single-precision%29)))

(fn StartSprint
  (params (CharacterMovement :type Character%20Movement%20Component%20Object%20Reference))
  (if (not (Variables|Default|GetisSprinting))
    (Variables|Default|SetisSprinting true)
    (Variables|/Script/Engine.CharacterMovementComponent|SetMaxWalkSpeed CharacterMovement (Variables|Default|GetSprintSpeed))))

(fn StopSprint
  (params (CharacterMovement :type Character%20Movement%20Component%20Object%20Reference))
  (if (Variables|Default|GetisSprinting)
    (Variables|Default|SetisSprinting false)
    (Variables|/Script/Engine.CharacterMovementComponent|SetMaxWalkSpeed CharacterMovement (Variables|Default|GetWalkSpeed))))